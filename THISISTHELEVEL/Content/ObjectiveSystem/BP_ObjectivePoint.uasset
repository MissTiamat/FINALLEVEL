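; BP_ObjectivePoint is a trigger actor that shows an objective notification when the player character enters its box, sized in the construction script.
; It creates a WBP_Objective widget on BeginPlay, then on first overlap plays a sound, fades the widget in and out, and flags the objective in progress.
; CompletedObjective reuses the widget to show a completion title with a success sound and the same timed fade.
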(event OnComponentBeginOverlap(ObjectiveBox)
  (params (OverlappedComponent :type Primitive%20Component%20Object%20Reference) (OtherActor :type Actor%20Object%20Reference) (OtherComp :type Primitive%20Component%20Object%20Reference) (OtherBodyIndex :type Integer) (bFromSweep :type Boolean) (SweepResult :type Hit%20Result%20Structure%20%28by%20ref%29))
  (bind _wbp_objecivewidgetref (Variables|Default|GetWBP_ObjeciveWidgetRef))
  (bind _wbp_objecivewidgetref_2 (Variables|Default|GetWBP_ObjeciveWidgetRef))
  (bind _objectivefade (Variables|/Game/ObjectiveSystem/WBP_Objective.WBP_Objective_C|GetObjectiveFade _wbp_objecivewidgetref))
  (if (== OtherActor (Game|GetPlayerCharacter 0))
    (Utilities|FlowControl|DoOnce false
      (:Completed
        (Variables|/Game/ObjectiveSystem/WBP_Objective.WBP_Objective_C|SetObjectiveTitleText _wbp_objecivewidgetref_2 (Variables|Default|GetObjective%20Title%20Text))
        (Variables|/Game/ObjectiveSystem/WBP_Objective.WBP_Objective_C|SetObjectiveTitleText _wbp_objecivewidgetref_2 (Variables|Default|GetObjective%20Title%20Text))
        (Audio|PlaySound2D "/Game/ObjectiveSystem/objectivesound.objectivesound" 1.0 1.0 0.0 0 0)
        (UserInterface|Viewport|AddtoViewport _wbp_objecivewidgetref 0)
        (UserInterface|Animation|PlayAnimation _wbp_objecivewidgetref _objectivefade 0.0 1 "Forward" 1.0 false)
        (Utilities|FlowControl|Delay 5.0)
        (UserInterface|Animation|PlayAnimation _wbp_objecivewidgetref _objectivefade 0.0 1 "Reverse" 1.0 false)
        (Variables|Default|SetObjectiveInProgress? true)))))

(event Custom|Completed%20Objective
  (bind _wbp_objecivewidgetref (Variables|Default|GetWBP_ObjeciveWidgetRef))
  (bind _objectivefade (Variables|/Game/ObjectiveSystem/WBP_Objective.WBP_Objective_C|GetObjectiveFade _wbp_objecivewidgetref))
  (Variables|/Game/ObjectiveSystem/WBP_Objective.WBP_Objective_C|SetObjectiveTitleText (Variables|Default|GetWBP_ObjeciveWidgetRef) "Completed Objective")
  (Audio|PlaySound2D "/Game/ObjectiveSystem/Successsound.Successsound" 1.0 1.0 0.0 0 0)
  (UserInterface|Animation|PlayAnimation _wbp_objecivewidgetref _objectivefade 0.0 1 "Forward" 1.0 false)
  (Utilities|FlowControl|Delay 3.0)
  (UserInterface|Animation|PlayAnimation _wbp_objecivewidgetref _objectivefade 0.0 1 "Reverse" 1.0 false))

(event EventBeginPlay
  (bind _returnvalue (UserInterface|CreateWidget "/Game/ObjectiveSystem/WBP_Objective.WBP_Objective_C" 0 (Variables|Default|GetObjective%20Title%20Text) (Variables|Default|GetObjective%20Content%20Text)))
  (Variables|Default|SetWBP_ObjeciveWidgetRef _returnvalue))

(fn ConstructionScript
  (Components|Box|SetBoxExtent (Variables|Default|GetObjective%20Box) (Variables|Default|GetObjective%20Box%20Size) true))