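; BP_Objective is a trigger-volume objective that shows a task on screen when the player reaches it.
; It creates a WB_Objective widget at BeginPlay, and the player's first overlap with the box fills in name and description, adds it to the viewport and animates it forward.
; A Completed event waits briefly, changes the name to a completion message, reverses the animation and sets the CompletedObjective flag.
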(event OnComponentBeginOverlap(Box)
  (params (OverlappedComponent :type Primitive%20Component%20Object%20Reference) (OtherActor :type Actor%20Object%20Reference) (OtherComp :type Primitive%20Component%20Object%20Reference) (OtherBodyIndex :type Integer) (bFromSweep :type Boolean) (SweepResult :type Hit%20Result%20Structure%20%28by%20ref%29))
  (bind _wb_objective (Variables|Default|GetWB_Objective))
  (if (== OtherActor (Game|GetPlayerCharacter 0))
    (Utilities|FlowControl|DoOnce false
      (:Completed
        (Variables|/Game/NewObjectiveSys/WB_Objective.WB_Objective_C|SetObjective_Desc _wb_objective (Variables|Default|GetObjective%20Desc))
        (Variables|/Game/NewObjectiveSys/WB_Objective.WB_Objective_C|SetObjective_Name _wb_objective (Variables|Default|GetObjective%20Name))
        (Default|ObjectiveAnim _wb_objective "Forward")
        (UserInterface|Viewport|AddtoViewport (Variables|Default|GetWB_Objective) 0)
        (Variables|Default|SetCompleted_Objective false)))))

(event Custom|Completed
  (bind _wb_objective (Variables|Default|GetWB_Objective))
  (Utilities|FlowControl|Delay 3.0)
  (Variables|/Game/NewObjectiveSys/WB_Objective.WB_Objective_C|SetObjective_Name _wb_objective "Completed Task!")
  (Default|ObjectiveAnim _wb_objective "Reverse")
  (Variables|Default|SetCompleted_Objective true))

(event EventBeginPlay
  (bind _returnvalue (UserInterface|CreateWidget "/Game/NewObjectiveSys/WB_Objective.WB_Objective_C" 0 (Variables|Default|GetObjective%20Name) (Variables|Default|GetObjective%20Desc)))
  (Variables|Default|SetWB_Objective _returnvalue))

(fn ConstructionScript)